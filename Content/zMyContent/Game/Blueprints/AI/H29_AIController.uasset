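; H29_AIController is an AI controller for team-based bots that runs their behavior tree and tells them where the enemy base is.
; BeginPlay runs H29_Base_AI_BT, noted as a debug start because the tree is assigned on AI_spawn.
; SetEnemyBasePos uses Team to index into all TeamSpawnPoint actors, relying on their returned order, and writes the opposing one's location to the EnemyBasePos blackboard key.
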(event EventBeginPlay
  ;[1 1 1] For debug, the tree gets assigned on AI_spawn
  (AI|RunBehaviorTree "/Game/zMyContent/Game/Blueprints/AI/H29_Base_AI_BT.H29_Base_AI_BT"))

(fn ConstructionScript)

(fn SetEnemyBasePos
  (bind _outactors (Actor|GetAllActorsOfClass "/Game/zMyContent/Game/Blueprints/Actors/TeamSpawnPoint.TeamSpawnPoint_C"))
  (switch Utilities|FlowControl|Switch|SwitchonTeams (Variables|Default|GetTeam)
    (:NewEnumerator0
      (LocalVariables|SetEnemyBasePos 1))
    (:NewEnumerator1
      (LocalVariables|SetEnemyBasePos 0)))
  (AI|Components|Blackboard|SetValueasVector (AI|GetBlackboard 0) (Utilities|Name|MakeLiteralName "EnemyBasePos") (Transformation|GetActorLocation (Utilities|Array|Get(acopy) _outactors (LocalVariables|GetEnemyBasePos)))))