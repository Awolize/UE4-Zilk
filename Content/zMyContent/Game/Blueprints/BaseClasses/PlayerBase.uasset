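; PlayerBase is a damageable base actor that tracks Health and an Alive state.
; Incoming damage subtracts from Health and clears Alive once Health reaches zero or below.
; Alive's RepNotify passes the actor's first tag to UpdateBaseState on player controller 0, cast to GamePlayPlayerController, identifying which base changed.
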(event Game|Damage|EventAnyDamage
  (params (Damage :type Float%20%28single-precision%29) (DamageType :type Damage%20Type%20Object%20Reference) (InstigatedBy :type Controller%20Object%20Reference) (DamageCauser :type Actor%20Object%20Reference))
  (bind _output_get (Variables|Default|SetHealth (- (Variables|Default|GetHealth) Damage)))
  (if (<= _output_get 0.0)
    (Variables|Default|SetAlive false)))

(fn ConstructionScript)

(fn OnRepAlive
  (Default|UpdateBaseState (.AsGame%20Play%20Player%20Controller (Utilities|Casting|CastToGamePlayPlayerController (Game|GetPlayerController 0))) (Utilities|Array|Get(acopy) (Variables|Actor|GetTags))))