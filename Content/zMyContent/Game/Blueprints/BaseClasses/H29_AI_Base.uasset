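; Base AI unit character for a team-based game that attacks enemy units and bases within a range sphere.
; Range overlaps filter by team tag, maintain an enemy list with bases pushed to the front, and set the EnemyInRange blackboard key.
; Tick attacks when not reloading, with separate damage for bases, while a looping timer clears the reload flag.
; Damage reduces health, destroying the unit at zero, and a RepNotify refreshes the health label.
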(event OnComponentBeginOverlap(RangeHitBox)
  (params (OverlappedComponent :type Primitive%20Component%20Object%20Reference) (OtherActor :type Actor%20Object%20Reference) (OtherComp :type Primitive%20Component%20Object%20Reference) (OtherBodyIndex :type Integer) (bFromSweep :type Boolean) (SweepResult :type Hit%20Result%20Structure%20%28by%20ref%29))
  ;[1 1 1] Event Overlap / Range
  (bind _isenemy (CallFunction|CheckifEnemy OtherActor))
  (if _isenemy
    (if (Utilities|DoesObjectImplementInterface OtherActor "/Game/zMyContent/Game/Blueprints/AI/IsUnitInterface.IsUnitInterface_C")
      (Utilities|Array|AddUnique (Variables|Default|GetEnemyArray) OtherActor)
      (CallFunction|SetBlackboardKeyEnemyinRange)
      (elif (Actor|ActorHasTag OtherActor "Base")
        (CallFunction|PushFront OtherActor)
        (CallFunction|SetBlackboardKeyEnemyinRange)))))

(event OnComponentEndOverlap(RangeHitBox)
  (params (OverlappedComponent :type Primitive%20Component%20Object%20Reference) (OtherActor :type Actor%20Object%20Reference) (OtherComp :type Primitive%20Component%20Object%20Reference) (OtherBodyIndex :type Integer))
  ;[1 1 1] Event Overlap / Range
  (Utilities|Array|RemoveItem (Variables|Default|GetEnemyArray) OtherActor)
  (CallFunction|SetBlackboardKeyEnemyinRange)
  (if (== (Utilities|Array|Length (Variables|Default|GetEnemyArray)) 0)
    _))

(event Custom|ShowRange
  ;[1 1 1] ShowRange
  (Rendering|ToggleVisibility (Variables|Default|GetRangeHitBox) false))

(event Custom|UpdateCharacter
  ;[1 1 1] Update all the Players
  (Rendering|Components|TextRender|SetText (Variables|Default|GetLabel) (Utilities|Text|ToText(Float) (Variables|UnitStat|GetHealthPoints) "HalfToEven")))

(event Custom|SetReload
  ;[1 1 1] Event BeginPlay
  (Variables|Default|SetReloading false))

(event Custom|RestartReloadTimer
  ;[1 1 1] Event BeginPlay
  (Utilities|Time|SetTimerbyEvent (delegate Custom|SetReload) (Variables|UnitStat|GetAttackSpeed) true))

(event EventBeginPlay
  ;[1 1 1] Event BeginPlay
  (Rendering|Components|TextRender|SetText (Variables|Default|GetLabel) (Utilities|Text|ToText(Float) (Variables|UnitStat|GetHealthPoints) "HalfToEven"))
  (Variables|/Script/Engine.CharacterMovementComponent|SetMaxWalkSpeed (Variables|Character|GetCharacterMovement) (Variables|UnitStat|GetMoveSpeed))
  (Components|Sphere|SetSphereRadius (Variables|Default|GetRangeHitBox) (Variables|UnitStat|GetRange) true)
  (Utilities|Time|SetTimerbyEvent (delegate Custom|SetReload) (Variables|UnitStat|GetAttackSpeed) true))

(event Game|Damage|EventAnyDamage
  (params (Damage :type Float%20%28single-precision%29) (DamageType :type Damage%20Type%20Object%20Reference) (InstigatedBy :type Controller%20Object%20Reference) (DamageCauser :type Actor%20Object%20Reference))
  ;[1 1 1] Event Damage Taken
  (CallFunction|DamageTaken Damage)
  (if (<= (Variables|UnitStat|GetHealthPoints) 0.0)
    (Actor|DestroyActor)))

(event EventTick
  (params (DeltaSeconds :type Float%20%28single-precision%29))
  (bind _enemyarray (Variables|Default|GetEnemyArray))
  (bind _mesh (Variables|Character|GetMesh))
  (bind _output (Utilities|Array|Get(acopy) _enemyarray))
  ;[1 1 1] Attack
  (if (not (Variables|Default|GetReloading))
    (if (!= (Utilities|Array|Length (Variables|Default|GetEnemyArray)) 0)
      (if (Actor|ActorHasTag _output "Base")
        (Game|Damage|ApplyDamage _output (Variables|UnitStat|GetBaseDamage) 0 0)
        (else
          (Game|Damage|ApplyDamage 0 (Variables|UnitStat|GetAttackDamage) 0 0)))
      (CallFunction|RestartReloadTimer)
      (Variables|Default|SetReloading true)
      (Audio|SpawnSound2D "/Engine/VREditor/Sounds/UI/Gizmo_Handle_Clicked.Gizmo_Handle_Clicked" 1.0 1.0 0.0 0)
      (Components|Animation|PlayAnimation _mesh "/Game/Mannequin/Animations/ThirdPerson_Jump.ThirdPerson_Jump" false)
      (Utilities|FlowControl|Delay 0.1)
      (Components|SkeletalMesh|SetAnimInstanceClass _mesh "/Game/Mannequin/Animations/ThirdPerson_AnimBP.ThirdPerson_AnimBP_C"))))

(fn ConstructionScript)

(fn CheckifEnemy
  (params (OverlappingActor :type Actor%20Object%20Reference))
  (return (not (or (and (Actor|ActorHasTag OverlappingActor "Team1") (Actor|ActorHasTag "Team1")) (and (Actor|ActorHasTag "Team2") (Actor|ActorHasTag OverlappingActor "Team2"))))))

(fn SetBlackboardKeyEnemyinRange
  (bind _returnvalue (Utilities|Name|MakeLiteralName "EnemyInRange"))
  (bind _returnvalue_2 (AI|GetBlackboard 0))
  (Utilities|IsValid _returnvalue_2
    (:Is%20Valid
      (if (!= 0 (Utilities|Array|Length (Variables|Default|GetEnemyArray)))
        (AI|Components|Blackboard|SetValueasBool _returnvalue_2 _returnvalue true)
        (else
          (AI|Components|Blackboard|SetValueasBool _returnvalue_2 _returnvalue false))))))

(fn DamageTaken
  (params (IncomingDamage :type Float%20%28single-precision%29))
  (Variables|UnitStat|SetHealthPoints (- (Variables|UnitStat|GetHealthPoints) IncomingDamage)))

(fn OnRepHealthPoints
  (CallFunction|UpdateCharacter))

(fn PushFront
  (params (PushFrontActor :type Actor%20Object%20Reference))
  (bind _temp (LocalVariables|Gettemp))
  (Utilities|Array|Add (LocalVariables|Gettemp) PushFrontActor)
  (for _array_element (Variables|Default|GetEnemyArray)
    (Utilities|Array|Add _temp _array_element))
  (Variables|Default|SetEnemyArray _temp))