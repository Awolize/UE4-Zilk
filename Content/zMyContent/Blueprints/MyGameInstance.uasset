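; Game Instance that manages menu flow, multiplayer sessions and error reporting.
; Show events lazily create and cache each menu or loading widget; a save-slot check opens either the main menu or first-time customization.
; LaunchLobby creates a named LAN or online session and opens LobbyLevel as listen server, while JoinServer joins search results.
; Session, network and travel failures feed one error dialog, with most network failures reported as lost host connection.
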(event Custom|ShowMainMenu
  ;[1 1 1] 1_MainMenuWidget and Enable Mouse Cursor
  (Utilities|IsValid (Variables|Widget|Get1_MainMenuWidget)
    (:Is%20Valid
      _)
    (:Is%20Not%20Valid
      (bind _returnvalue (UserInterface|CreateWidget "/Game/zMyContent/Menu/UMG/1_MainMenu.1_MainMenu_C" (Game|GetPlayerController 0)))
      (Variables|Widget|Set1_MainMenuWidget _returnvalue)))
  (UserInterface|Viewport|AddtoViewport (Variables|Widget|Get1_MainMenuWidget) 0)
  (Variables|/Script/Engine.PlayerController|SetbShowMouseCursor (Game|GetPlayerController 0) true))

(event Custom|ShowPlayMenu
  ;[1 1 1] 2_PlayGameWidget
  (Utilities|IsValid (Variables|Widget|Get2_PlayGameWidget)
    (:Is%20Valid
      _)
    (:Is%20Not%20Valid
      (bind _returnvalue (UserInterface|CreateWidget "/Game/zMyContent/Menu/UMG/2_PlayGame.2_PlayGame_C" (Game|GetPlayerController 0)))
      (Variables|Widget|Set2_PlayGameWidget _returnvalue)))
  (UserInterface|Viewport|AddtoViewport (Variables|Widget|Get2_PlayGameWidget) 0))

(event Custom|JoinServer
  (params (SessionToJoin :type Blueprint%20Session%20Result%20Structure))
  ;[1 1 1] JoinServer
  (CallFunction|ShowLoadingScreen)
  (|JoinSession (Game|GetPlayerController 0) SessionToJoin
    (:OnFailure
      (Utilities|DisplayErrorMessage "Failed to Join Session"))))

(event Custom|DestorySessionCaller
  (params (PlayerController :type Player%20Controller%20Object%20Reference))
  ;[1 1 1] Destroy Session
  (|DestroySession PlayerController))

(event Custom|SaveGameCheck
  ;[1 1 1] SaveGameCheck
  (bind _returnvalue (SaveGame|DoesSaveGameExist (Variables|Default|GetPlayerSettingsSave)))
  (if _returnvalue
    (CallFunction|ShowMainMenu)
    (Variables|Default|SetCreatedSaveFile true)
    (else
      (CallFunction|ShowCustomizationMenu)
      (Variables|/Script/Engine.PlayerController|SetbShowMouseCursor (Game|GetPlayerController 0) true))))

(event Custom|BackToMenu
  ;[1 1 1] Back to main menu
  (Viewport|RemoveAllWidgets)
  (CallFunction|ShowMainMenu))

(event Custom|DeleteSaveGame
  ;[1 1 1] Delete Save Game
  (SaveGame|DeleteGameinSlot (Variables|Default|GetPlayerSettingsSave))
  (Development|PrintString "Save Deleted"))

(event Custom|ShowHostGameMenu
  ;[1 1 1] 3_HostGameWidget
  (Utilities|IsValid (Variables|Widget|Get3_HostGameWidget)
    (:Is%20Valid
      _)
    (:Is%20Not%20Valid
      (bind _returnvalue (UserInterface|CreateWidget "/Game/zMyContent/Menu/UMG/3_HostGame.3_HostGame_C" (Game|GetPlayerController 0)))
      (Variables|Widget|Set3_HostGameWidget _returnvalue)))
  (UserInterface|Viewport|AddtoViewport (Variables|Widget|Get3_HostGameWidget) 0))

(event Custom|UserOptionShowFPS
  ;[1 1 1] UserOptionShowFPS
  (if (Variables|UserSettings|GetUserEnabledFPS)
    (Development|ExecuteConsoleCommand "stat fps" (Game|GetPlayerController 0))))

(event Custom|ShowStatsWidget
  ;[1 1 1] Comment
  (Utilities|IsValid (Variables|Widget|Get2_ShowStatsWidget)
    (:Is%20Valid
      _)
    (:Is%20Not%20Valid
      (bind _returnvalue (UserInterface|CreateWidget "/Game/zMyContent/Menu/UMG/2_Stats.2_Stats_C" (Game|GetPlayerController 0)))
      (Variables|Widget|Set2_ShowStatsWidget _returnvalue)))
  (UserInterface|Viewport|AddtoViewport (Variables|Widget|Get2_ShowStatsWidget) 0))

(event Custom|ShowCustomizationMenu
  ;[1 1 1] 2_CustomizationWidget
  (Utilities|IsValid (Variables|Widget|Get2_ShowCustomizationWidget)
    (:Is%20Valid
      _)
    (:Is%20Not%20Valid
      (bind _returnvalue (UserInterface|CreateWidget "/Game/zMyContent/Menu/UMG/2_Customization.2_Customization_C" (Game|GetPlayerController 0)))
      (Variables|Widget|Set2_ShowCustomizationWidget _returnvalue)))
  (UserInterface|Viewport|AddtoViewport (Variables|Widget|Get2_ShowCustomizationWidget) 0))

(event Custom|ShowServerBrowserMenu
  ;[1 1 1] 3_SearchGameWidget
  (Utilities|IsValid (Variables|Widget|Get3_ServerBrowserWidget)
    (:Is%20Valid
      _)
    (:Is%20Not%20Valid
      (bind _returnvalue (UserInterface|CreateWidget "/Game/zMyContent/Menu/UMG/3_SearchGame.3_SearchGame_C" (Game|GetPlayerController 0)))
      (Variables|Widget|Set3_ServerBrowserWidget _returnvalue)))
  (UserInterface|Viewport|AddtoViewport (Variables|Widget|Get3_ServerBrowserWidget) 0))

(event Custom|ShowOptionsWidget
  ;[1 1 1] Comment
  (Utilities|IsValid (Variables|Widget|Get2_ShowOptionsWidget)
    (:Is%20Valid
      _)
    (:Is%20Not%20Valid
      (bind _returnvalue (UserInterface|CreateWidget "/Game/zMyContent/Menu/UMG/2_Options.2_Options_C" (Game|GetPlayerController 0)))
      (Variables|Widget|Set2_ShowOptionsWidget _returnvalue)))
  (UserInterface|Viewport|AddtoViewport (Variables|Widget|Get2_ShowOptionsWidget) 0))

(event Custom|LaunchLobby
  (params (MaxPlayers :type Integer) (LAN :type Boolean) (ServerName :type Text))
  ;[1 1 1] LaunchLobby
  (Variables|ServerSettings|SetServerName ServerName)
  (Variables|ServerSettings|SetMaxPlayers MaxPlayers)
  (CallFunction|ShowLoadingScreen)
  (|AdvancedSession (Utilities|Array|MakeArray (Class|AdvancedSessionsLibrary|MakeLiteralSessionPropertyString "ServerName" (Utilities|String|ToString(Text) (Variables|ServerSettings|GetServerName)))) (Game|GetPlayerController 0) (Variables|ServerSettings|GetMaxPlayers) 0 LAN true false true true false false false true
    (:OnSuccess
      (Game|OpenLevel(byName) "LobbyLevel" true "listen")
      (Development|PrintString (Utilities|String|Append "Server name: " (Utilities|String|ToString(Text) (Variables|ServerSettings|GetServerName)))))
    (:OnFailure
      (Utilities|DisplayErrorMessage "Failed to Create Session"))))

(event Custom|ShowLoadingScreen
  ;[1 1 1] ShowLoadingScreen
  (Utilities|IsValid (Variables|Widget|GetLoadingScreenWidget)
    (:Is%20Valid
      _)
    (:Is%20Not%20Valid
      (bind _returnvalue (UserInterface|CreateWidget "/Game/zMyContent/Blueprints/LoadingScreenWidget.LoadingScreenWidget_C" (Game|GetPlayerController 0)))
      (Variables|Widget|SetLoadingScreenWidget _returnvalue)))
  (UserInterface|Viewport|AddtoViewport (Variables|Widget|GetLoadingScreenWidget) 0))

(event EventHandleTravelError
  (params (FailureType :type ETravelFailure%20Enum :default "NoLevel"))
  ;[1 1 1] Handle Travel Errors
  (Utilities|DisplayErrorMessage (CallFunction|TravelErrortoString FailureType)))

(event EventHandleNetworkError
  (params (FailureType :type ENetworkFailure%20Enum :default "NetDriverAlreadyExists") (bIsServer :type Boolean))
  ;[1 1 1] Handle Network Errors
  (if bIsServer
    _
    (else
      _))
  (Utilities|DisplayErrorMessage (CallFunction|NetworkErrortoString FailureType)))

(fn NetworkErrortoString
  (params (FailureType :type ENetworkFailure%20Enum :default "NetDriverAlreadyExists"))
  (switch Utilities|FlowControl|Switch|SwitchonENetworkFailure FailureType
    (:NetDriverAlreadyExists
      (Variables|Default|SetErrorString "Error : Lost Connection to Host" :!label _label))
    (:NetDriverCreateFailure
      (goto _label))
    (:NetDriverListenFailure
      (goto _label))
    (:ConnectionLost
      (goto _label))
    (:ConnectionTimeout
      (Variables|Default|SetErrorString "Error : Connection Timed Out"))
    (:FailureReceived
      (goto _label))
    (:OutdatedClient
      (goto _label))
    (:OutdatedServer
      (goto _label))
    (:PendingConnectionFailure
      (goto _label))
    (:NetGuidMismatch
      (goto _label))
    (:NetChecksumMismatch
      (goto _label)))
  (return (Variables|Default|GetErrorString)))

(fn TravelErrortoString
  (params (FailureType :type ETravelFailure%20Enum :default "NoLevel"))
  (return (Utilities|String|Append "Error : Failed to Travel" (Utilities|String|EnumtoString FailureType))))