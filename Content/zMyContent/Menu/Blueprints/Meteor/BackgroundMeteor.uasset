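; BackgroundMeteor is a meteor actor, filed under the menu Blueprints, that slowly tumbles in place.
; Tick counts a timer down by delta time and, each time it drops below zero, adds a small random positive local rotation on all three axes and resets it.
; The very short timer allows at most one step per frame, so spin speed depends on frame rate.
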(event EventBeginPlay)

(event Collision|EventActorBeginOverlap
  (params (OtherActor :type Actor%20Object%20Reference)))

(event EventTick
  (params (DeltaSeconds :type Float%20%28single-precision%29))
  (bind _output_get (Variables|Default|SetTimer (- (Variables|Default|GetTimer) DeltaSeconds)))
  (if (< _output_get 0.0)
    (Transformation|AddActorLocalRotation (Math|Rotator|MakeRotator (Math|Random|RandomFloatinRange 0.1 0.2) (Math|Random|RandomFloatinRange 0.1 0.2) (Math|Random|RandomFloatinRange 0.1 0.2)) false false)
    (Variables|Default|SetTimer 0.01)))

(fn ConstructionScript)