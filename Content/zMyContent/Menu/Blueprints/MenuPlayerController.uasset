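; Player controller for the menu that applies display settings and handles debug-style shortcut keys for quitting, returning to the main menu and deleting the save.
; BeginPlay caps the frame rate, shows FPS stats and records the current window mode and desktop resolution.
; Display changes run through r.setRes console commands built from resolution plus a mode suffix.
; A KeepSettings widget follows each mode change, with events to keep new or restore old values.
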(event Custom|ChangeDisplayMode
  (params (DisplayType :type EWindowMode%20Enum :default "Fullscreen"))
  ;[1 1 1] Display Mode
  (bind _returnvalue (Settings|GetGameUserSettings))
  (Utilities|FlowControl|Sequence
    (:then_0
      (CallFunction|SaveEWindowMode (Class|GameUserSettings|GetFullscreenMode _returnvalue) false))
    (:then_1
      (CallFunction|SaveEWindowMode DisplayType true)
      (CallFunction|SetResolution (Variables|Default|GetResolution))
      (bind _returnvalue_2 (UserInterface|CreateWidget "/Game/zMyContent/Menu/UMG/2_Options/KeepSettings.KeepSettings_C" (Game|GetPlayerController 0)))
      (UserInterface|Viewport|AddtoViewport _returnvalue_2 0))))

(event Custom|KeepOldDisplaySettings
  ;[1 1 1] Display Mode
  (Variables|Default|SetDisplayMode (Variables|Default|GetOldDisplayMode))
  (CallFunction|SetResolution (Variables|Default|GetOldResolution)))

(event Custom|SetResolution
  (params (NewResolution :type Int%20Point%20Structure))
  (bind (_x _y) (Utilities|Struct|BreakIntPoint NewResolution))
  (bind _displaymode (Variables|Default|GetDisplayMode))
  (bind _returnvalue (Utilities|String|ToString(Integer) _x))
  (bind _returnvalue_2 (Utilities|String|ToString(Integer) _y))
  (bind _returnvalue_3 (Utilities|String|Append "r.setRes " _returnvalue "x" _returnvalue_2 _displaymode))
  ;[1 1 1] SetResolution
  (Variables|Default|SetResolution NewResolution)
  (Development|PrintString _returnvalue_3)
  (Development|ExecuteConsoleCommand _returnvalue_3 (Game|GetPlayerController 0))
  (bind _returnvalue_4 (Settings|GetGameUserSettings))
  (Class|GameUserSettings|SaveSettings _returnvalue_4))

(event Custom|KeepNewDisplaySettings
  ;[1 1 1] Display Mode
  (Variables|Default|SetOldResolution (Variables|Default|GetResolution))
  (Variables|Default|SetOldDisplayMode (Variables|Default|GetDisplayMode)))

(event Custom|SetFrameRate
  (params (NewFpsCap :type Float%20%28single-precision%29))
  ;[1 1 1] Set Frame Rate
  (bind _returnvalue (Settings|GetGameUserSettings))
  (Class|GameUserSettings|SetFrameRateLimit _returnvalue NewFpsCap)
  (Class|GameUserSettings|ApplyNonResolutionSettings _returnvalue))

(event EventBeginPlay
  ;[1 1 1] Event BeginPlay
  (CallFunction|SetFrameRate self 144.0)
  (Development|ExecuteConsoleCommand "stat fps" (Game|GetPlayerController 0))
  (bind _returnvalue (Settings|GetGameUserSettings))
  (CallFunction|SaveEWindowMode (Class|GameUserSettings|GetFullscreenMode _returnvalue) true)
  (CallFunction|SaveEWindowMode (Class|GameUserSettings|GetFullscreenMode _returnvalue) false)
  (bind _output_get (Variables|Default|SetResolution (Class|GameUserSettings|GetDesktopResolution _returnvalue)))
  (Variables|Default|SetOldResolution _output_get))

(event Input|KeyboardEvents|O
  (params (Key :type Key%20Structure))
  ;[1 1 1] Call Delete Save Game
  (:Pressed
    (bind _asmy_game_instance (Utilities|Casting|CastToMyGameInstance (Game|GetGameInstance)))
    (Default|DeleteSaveGame _asmy_game_instance)))

(event Input|KeyboardEvents|Escape
  (params (Key :type Key%20Structure))
  ;[1 1 1] Exit game
  (:Pressed
    (Game|QuitGame 0 "Quit")))

(event Input|KeyboardEvents|B
  (params (Key :type Key%20Structure))
  ;[1 1 1] Back to main menu when "B" is pressed
  (:Pressed
    (Default|BacktoMenu (.AsMy%20Game%20Instance (Utilities|Casting|CastToMyGameInstance (Game|GetGameInstance))))))

(fn ConstructionScript)

(fn SaveEWindowMode
  (params (EWindowMode :type EWindowMode%20Enum :default "Fullscreen") (NewSettings? :type Boolean))
  (if NewSettings?
    (switch Utilities|FlowControl|Switch|SwitchonEWindowMode EWindowMode
      (:Fullscreen
        (Variables|Default|SetDisplayMode "f"))
      (:WindowedFullscreen
        (Variables|Default|SetDisplayMode "wf"))
      (:Windowed
        (Variables|Default|SetDisplayMode "w")))
    (else
      (switch Utilities|FlowControl|Switch|SwitchonEWindowMode EWindowMode
        (:Fullscreen
          (Variables|Default|SetOldDisplayMode "f"))
        (:WindowedFullscreen
          (Variables|Default|SetOldDisplayMode "wf"))
        (:Windowed
          (Variables|Default|SetOldDisplayMode "w")))))
  (return))